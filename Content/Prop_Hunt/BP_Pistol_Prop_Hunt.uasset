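; Pistol weapon for the hunter in the Prop Hunt mode, handling shooting input and fire feedback.
; On BeginPlay it caches the owning BP_Hunter and adds the pistol's Enhanced Input mapping context to that hunter's player controller.
; Shooting traces from the Muzzle socket along the camera's forward vector with debug drawing, then plays a sound and arm montage.
; The trace result is unused, so shots apply no damage.
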(event `self.ReceiveBeginPlay`
  ;[1 1 1] Set up arme IMC
  (bind _asbp_hunter (cast `/Game/Prop_Hunt/BP_Hunter` (`self.GetOwner`)))
  (bind _output_get (set `self.As BP Hunter` _asbp_hunter))
  (bind _asbp_player_controller_prop_hunt (cast `/Game/Prop_Hunt/Input/BP_Player_Controller_Prop_Hunt` (`Pawn.GetController` _output_get)))
  (bind _returnvalue (pcsubsystem `EnhancedInputLocalPlayerSubsystem` _asbp_player_controller_prop_hunt))
  (`/Engine/EditorBlueprintResources/StandardMacros.IsValid` _returnvalue
    (:`Is Valid`
      (`EnhancedInputSubsystemInterface.AddMappingContext` _returnvalue "/Game/Prop_Hunt/Input/IMC_Pistol_Prop_Hunt.IMC_Pistol_Prop_Hunt" 1 (struct)))))

(event `EnhancedInput|/Game/Prop_Hunt/Input/IA_Shoot_Pop_Hunt`
  (params (ActionValue :type Boolean) (ElapsedSeconds :type "Float (double-precision)") (TriggeredSeconds :type "Float (double-precision)") (InputAction :type "InputAction Object Reference" :default "/Game/Prop_Hunt/Input/IA_Shoot_Pop_Hunt.IA_Shoot_Pop_Hunt"))
  (bind _returnvalue (`self.GetSocketLocation` "Muzzle"))
  (:`Triggered`
    (`KismetSystemLibrary.LineTraceSingle` :`Start` _returnvalue :`End` (+ _returnvalue (* (`self.GetForwardVector` (`/Game/Prop_Hunt/BP_Hunter.Camera` (`self.As BP Hunter`))) (`self.Shoot_Range`))) :`TraceChannel` "TraceTypeQuery1" :`DrawDebugType` "ForDuration")
    (`GameplayStatics.PlaySoundAtLocation` "/Game/FPWeapon/Audio/FirstPersonTemplateWeaponFire02.FirstPersonTemplateWeaponFire02" _returnvalue (struct) 1.0 1.0 0.0 null null null null)
    (`AnimInstance.Montage_Play` (`self.GetAnimInstance` (`/Game/Prop_Hunt/BP_Hunter.Arm` (`self.As BP Hunter`))) "/Game/FirstPersonArms/Animations/FP_Rifle_Shoot_Montage.FP_Rifle_Shoot_Montage" 1.0 "MontageLength" 0.0 true)))