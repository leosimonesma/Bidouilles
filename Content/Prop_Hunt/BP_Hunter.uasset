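; BP_Hunter is the hunter character for the Prop Hunt mode, providing basic player-controlled looking, walking and jumping.
; Enhanced Input actions drive it: look input feeds controller yaw and pitch, and move input moves it along the actor's right and forward vectors.
; The jump action starts a jump when pressed and stops it on completion.
; The Blueprint's graphs hold no hunting-specific logic, and its construction script is empty.
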(event `EnhancedInput|/Game/Prop_Hunt/Input/IA_Look_Prop_Hunt`
  (params (ActionValue :type "Vector2D Structure") (ElapsedSeconds :type "Float (double-precision)") (TriggeredSeconds :type "Float (double-precision)") (InputAction :type "InputAction Object Reference" :default "/Game/Prop_Hunt/Input/IA_Look_Prop_Hunt.IA_Look_Prop_Hunt"))
  (bind (_x _y) (`KismetMathLibrary.BreakVector2D` ActionValue))
  ;[1 1 1] Camera Movement
  (:`Triggered`
    (bind _result (`/Engine/EditorBlueprintResources/StandardMacros.NegateFloat` _x)
      (:`  `
        (`self.AddControllerYawInput` _result)
        (`self.AddControllerPitchInput` _y)))))

(event `EnhancedInput|/Game/Prop_Hunt/Input/IA_Move_Prop_Hunt`
  (params (ActionValue :type "Vector2D Structure") (ElapsedSeconds :type "Float (double-precision)") (TriggeredSeconds :type "Float (double-precision)") (InputAction :type "InputAction Object Reference" :default "/Game/Prop_Hunt/Input/IA_Move_Prop_Hunt.IA_Move_Prop_Hunt"))
  (bind (_x _y) (`KismetMathLibrary.BreakVector2D` ActionValue))
  ;[1 1 1] Déplacements
  (:`Triggered`
    (`self.AddMovementInput` (`self.GetActorRightVector`) _x)
    (`self.AddMovementInput` (`self.GetActorForwardVector`) _y)))

(event `EnhancedInput|/Game/Prop_Hunt/Input/IA_Jump_Prop_Hunt`
  (params (ActionValue :type Boolean) (ElapsedSeconds :type "Float (double-precision)") (TriggeredSeconds :type "Float (double-precision)") (InputAction :type "InputAction Object Reference" :default "/Game/Prop_Hunt/Input/IA_Jump_Prop_Hunt.IA_Jump_Prop_Hunt"))
  ;[1 1 1] Jumping
  (:`Started`
    (`self.Jump`))
  (:`Completed`
    (`self.StopJumping`)))

(fn `UserConstructionScript`)